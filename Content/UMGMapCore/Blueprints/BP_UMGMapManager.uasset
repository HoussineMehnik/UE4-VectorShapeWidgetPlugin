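; Manager actor for a UMG map that keeps the registry of map markers and provides the world map's origin, size, transform and yaw.
; Any object implementing the marker interface can register or unregister, and each change fires a registered or removed notification.
; It can also construct standalone marker objects from init data, rejecting invalid or duplicate tags, which serve as lookup keys.
; Map bounds come from a referenced vector shape actor.
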(event Custom|Register%20Marker%20Object
  (params (New%20Marker%20Object :type Object%20Object%20Reference))
  ;[1 0.7582 0] Register/Unregister existing makers ( Object , Component, Actors ) : Any object type implemeting BP_MarkerObjectInterface
  (Utilities|IsValid New%20Marker%20Object
    (:Is%20Valid
      (if (not (Utilities|Array|ContainsItem (Variables|Default|GetMarker%20Objects%20List) New%20Marker%20Object))
        (Utilities|Array|Add (Variables|Default|GetMarker%20Objects%20List) New%20Marker%20Object)
        (Default|CallOnMarkerObjectRegistered New%20Marker%20Object)))))

(event Custom|Create%20New%20Marker%20Object
  (params (Init%20Data :type Struct%20Marker%20Data%20Structure))
  (bind _uniquetag (Utilities|Struct|BreakStruct_MarkerData Init%20Data))
  ;[0.4844 0.2739 0.1299] Create New Marker Object :
  ; Can be used for example , to indicate a static point based on it location ,
  ; here the unique tag is used to find the created object if we haven't stored a refrence of it
  (bind _return_value (CallFunction|MarkerTagIsValid _uniquetag))
  (if _return_value
    (bind _return_value_ (CallFunction|GetRegisteredMarkerObjectIndexbyTag _uniquetag))
    (if (== _return_value_ -1)
      (bind _returnvalue (Game|ConstructObjectfromClass "/Game/UMGMapCore/Blueprints/BP_MarkerObject.BP_MarkerObject_C" self Init%20Data))
      (Utilities|IsValid _returnvalue
        (:Is%20Valid
          (CallFunction|RegisterMarkerObject _returnvalue)))
      (else
        (Development|PrintString "Failed To Create New Marker : TAG ALREADY REGISTERED" true true "(R=1.000000,G=0.000000,B=0.000000,A=1.000000)")))
    (else
      (Development|PrintString "Failed To Create New Marker : INVALID TAG" true true "(R=1.000000,G=0.000000,B=0.000000,A=1.000000)"))))

(event Custom|Unregister%20Marker%20Object
  (params (Marker%20Object :type BP%20Marker%20Component%20Object%20Reference))
  ;[1 0.7582 0] Register/Unregister existing makers ( Object , Component, Actors ) : Any object type implemeting BP_MarkerObjectInterface
  (Utilities|IsValid Marker%20Object
    (:Is%20Valid
      (bind _returnvalue (Utilities|Array|RemoveItem (Variables|Default|GetMarker%20Objects%20List) Marker%20Object))
      (if _returnvalue
        (Default|CallOnMarkerObjectRemoved Marker%20Object)))))

(fn ConstructionScript
  (Editor|LockScaleandRotation))

(fn LockScaleandRotation
  (Transformation|SetActorRotation (Math|Rotator|MakeRotator 0.0 0.0 (.Yaw (Math|Rotator|BreakRotator (Transformation|GetActorRotation)))))
  (Transformation|SetActorScale3D "1.000000,1.000000,1.000000"))

(fn GetRegisteredMarkerObjectbyTag
  (params (Target%20Tag :type String))
  (Utilities|FlowControl|Sequence
    (:then_0
      (LocalVariables|SetOut%20Marker%20Object 0)
      (bind _return_value (CallFunction|MarkerTagIsValid Target%20Tag))
      (if _return_value
        (bind _array_element (Utilities|Array|ForEachLoopwithBreak (Variables|Default|GetMarker%20Objects%20List) :!label _label)
          (:LoopBody
            (Utilities|IsValid _array_element
              (:Is%20Valid
                (bind _return_value_2 (Class|BPMarkerObjectInterface|GetMarkerTag(Message) _array_element))
                (if (Utilities|Enum|Equal(Enum) _return_value_2 Target%20Tag)
                  (LocalVariables|SetOut%20Marker%20Object _array_element)
                  (goto _label Break))))))))
    (:then_1
      (return (LocalVariables|GetOut%20Marker%20Object)))))

(fn GetRegisteredMarkerObjectIndexbyTag
  (params (Target%20Tag :type String))
  (Utilities|FlowControl|Sequence
    (:then_0
      (LocalVariables|SetOut%20Index -1)
      (bind (_array_element _array_index) (Utilities|Array|ForEachLoopwithBreak (Variables|Default|GetMarker%20Objects%20List) :!label _label)
        (:LoopBody
          (Utilities|IsValid _array_element
            (:Is%20Valid
              (bind _return_value (Class|BPMarkerObjectInterface|GetMarkerTag(Message) _array_element))
              (if (Utilities|Enum|Equal(Enum) _return_value Target%20Tag)
                (LocalVariables|SetOut%20Index _array_index)
                (goto _label Break)))))))
    (:then_1
      (return (LocalVariables|GetOut%20Index)))))

(fn GetWorldMapOrigin
  (Utilities|IsValid (Variables|Default|GetVector%20Shape%20Actor)
    (:Is%20Valid
      (return (Transformation|GetActorLocation (Variables|Default|GetVector%20Shape%20Actor))))
    (:Is%20Not%20Valid
      (Development|PrintString "Can't get location : Vector Actor Reference not valid" true true "(R=1.000000,G=0.000000,B=0.030547,A=1.000000)")
      (return "0, 0, 0"))))

(fn GetWorldMapSize
  (Utilities|IsValid (Variables|Default|GetVector%20Shape%20Actor)
    (:Is%20Valid
      (return (Variables|/Script/VectorShape.VectorShapeActor|GetWorldSize (Variables|Default|GetVector%20Shape%20Actor))))
    (:Is%20Not%20Valid
      (Development|PrintString "Can't get size : Vector Actor Reference not valid" true true "(R=1.000000,G=0.000000,B=0.030547,A=1.000000)")
      (return ""))))

(fn GetWorldMapTransform
  (bind _vector_shape_actor (Variables|Default|GetVector%20Shape%20Actor))
  (Utilities|IsValid (Variables|Default|GetVector%20Shape%20Actor)
    (:Is%20Valid
      (return (Math|Transform|MakeTransform (Transformation|GetActorLocation _vector_shape_actor) (Math|Rotator|MakeRotator 0.0 0.0 (.Yaw (Math|Rotator|BreakRotator (Transformation|GetActorRotation _vector_shape_actor)))))))
    (:Is%20Not%20Valid
      (Development|PrintString "Can't get location : Vector Actor Reference not valid" true true "(R=1.000000,G=0.000000,B=0.030547,A=1.000000)")
      (return ""))))

(fn GetWorldMapRotationAngle
  (Utilities|IsValid (Variables|Default|GetVector%20Shape%20Actor)
    (:Is%20Valid
      (return (.Yaw (Math|Rotator|BreakRotator (Transformation|GetActorRotation (Variables|Default|GetVector%20Shape%20Actor))))))
    (:Is%20Not%20Valid
      (Development|PrintString "Can't get location : Vector Actor Reference not valid" true true "(R=1.000000,G=0.000000,B=0.030547,A=1.000000)")
      (return 0.0))))