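; Blueprint interface for map marker objects in the UMGMapCore utilities, defining the contract for reading and changing a marker.
; Getters expose status, tag, icon object, color, opacity, world position, rotation angle and scale, with matching setters for most of these.
; It also declares a bulk data override, a status update, and a flag for hiding the marker when it goes out of range.
; All functions are empty stubs, leaving the behavior to implementers.
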(fn GetMarkerStatus
  (return "NewEnumerator0"))

(fn GetMarkerTag
  (return ""))

(fn OverrideMarkerData
  (params (New%20Data :type Struct%20Marker%20Data%20Structure)))

(fn SetMarkerIconObject
  (params (New%20Icon%20Object :type Object%20Object%20Reference)))

(fn SetMarkerColor
  (params (New%20Color :type Linear%20Color%20Structure)))

(fn SetMarkerOpacity
  (params (New%20Opacity :type Float%20%28single-precision%29)))

(fn SetMarkerWorldLocation
  (params (New%20Location :type Vector)))

(fn SetMarkerRotationAngle
  (params (New%20Rotation%20Angle :type Float%20%28single-precision%29)))

(fn SetMarkerScale
  (params (New%20Scale :type Float%20%28single-precision%29)))

(fn UpdateMarkerStatus
  (params (New%20Status :type Enum_MarkerStatus%20Enum :default "NewEnumerator0")))

(fn IsMarkerHidenwhenGettingOutOfRange
  (return false))

(fn SetMarkerHiddenwhenGettingOutOfRange
  (params (Value :type Boolean)))

(fn GetMarkerIconObject
  (return 0))

(fn GetMarkerIconColor
  (return ""))

(fn GetMarkerIconOpacity
  (return 0.0))

(fn GetMarkerWorldPosition
  (return "0, 0, 0"))

(fn GetMarkerRotationAngle
  (return 0.0))

(fn GetMarkerScale
  (return 0.0))