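; BP_MarkerObject is the data object for a single map marker in the UMG map system.
; It stores one MarkerData struct covering icon, color, opacity, transform, status, tag and out-of-range hiding.
; Marker interface events overwrite the struct whole or per field, clamping opacity, rotation angle and scale, while getter functions expose the fields.
; The tag has a getter but no individual setter, and no drawing happens here.
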(event EventSetMarkerWorldLocation
  (params (New%20Location :type Vector :default "0, 0, 0"))
  ;[0 0.2854 1] Marker Object Interface Events
  (Utilities|Struct|SetmembersinStruct_MarkerData (Variables|Default|GetMarker%20Data) New%20Location))

(event EventOverrideMarkerData
  (params (New%20Data :type Struct%20Marker%20Data%20Structure))
  ;[0 0.2854 1] Marker Object Interface Events
  (Variables|Default|SetMarker%20Data New%20Data))

(event EventUpdateMarkerStatus
  (params (New%20Status :type Enum_MarkerStatus%20Enum :default "NewEnumerator0"))
  ;[0 0.2854 1] Marker Object Interface Events
  (Utilities|Struct|SetmembersinStruct_MarkerData (Variables|Default|GetMarker%20Data) New%20Status))

(event EventSetMarkerIconObject
  (params (New%20Icon%20Object :type Object%20Object%20Reference))
  ;[0 0.2854 1] Marker Object Interface Events
  (Utilities|Struct|SetmembersinStruct_MarkerData (Variables|Default|GetMarker%20Data) New%20Icon%20Object))

(event EventSetMarkerColor
  (params (New%20Color :type Linear%20Color%20Structure))
  ;[0 0.2854 1] Marker Object Interface Events
  (Utilities|Struct|SetmembersinStruct_MarkerData (Variables|Default|GetMarker%20Data) New%20Color))

(event EventSetMarkerOpacity
  (params (New%20Opacity :type Float%20%28single-precision%29))
  ;[0 0.2854 1] Marker Object Interface Events
  (Utilities|Struct|SetmembersinStruct_MarkerData (Variables|Default|GetMarker%20Data) (Math|Float|Clamp(Float) New%20Opacity)))

(event EventSetMarkerRotationAngle
  (params (New%20Rotation%20Angle :type Float%20%28single-precision%29))
  ;[0 0.2854 1] Marker Object Interface Events
  (Utilities|Struct|SetmembersinStruct_MarkerData (Variables|Default|GetMarker%20Data) (Math|Float|ClampAngle New%20Rotation%20Angle -1.8e+02 1.8e+02)))

(event EventSetMarkerScale
  (params (New%20Scale :type Float%20%28single-precision%29))
  ;[0 0.2854 1] Marker Object Interface Events
  (Utilities|Struct|SetmembersinStruct_MarkerData (Variables|Default|GetMarker%20Data) (Math|Float|Clamp(Float) New%20Scale 0.0 1e+01)))

(event EventSetMarkerHiddenwhenGettingOutOfRange
  (params (Value :type Boolean))
  ;[0 0.2854 1] Marker Object Interface Events
  (Utilities|Struct|SetmembersinStruct_MarkerData (Variables|Default|GetMarker%20Data) Value))

(fn GetMarkerIconColor
  (return (Utilities|Struct|BreakStruct_MarkerData (Variables|Default|GetMarker%20Data))))

(fn GetMarkerIconObject
  (return (Utilities|Struct|BreakStruct_MarkerData (Variables|Default|GetMarker%20Data))))

(fn GetMarkerIconOpacity
  (return (Utilities|Struct|BreakStruct_MarkerData (Variables|Default|GetMarker%20Data))))

(fn GetMarkerRotationAngle
  (return (Utilities|Struct|BreakStruct_MarkerData (Variables|Default|GetMarker%20Data))))

(fn GetMarkerScale
  (return (Utilities|Struct|BreakStruct_MarkerData (Variables|Default|GetMarker%20Data))))

(fn GetMarkerStatus
  (return (Utilities|Struct|BreakStruct_MarkerData (Variables|Default|GetMarker%20Data))))

(fn GetMarkerTag
  (return (Utilities|Struct|BreakStruct_MarkerData (Variables|Default|GetMarker%20Data))))

(fn GetMarkerWorldPosition
  (return (Utilities|Struct|BreakStruct_MarkerData (Variables|Default|GetMarker%20Data))))

(fn IsMarkerHidenwhenGettingOutOfRange
  (return (Utilities|Struct|BreakStruct_MarkerData (Variables|Default|GetMarker%20Data))))