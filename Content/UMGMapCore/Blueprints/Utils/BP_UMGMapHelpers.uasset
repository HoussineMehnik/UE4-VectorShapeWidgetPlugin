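; Helper function library for the UMG map system, offering shared utility functions.
; It validates marker tags, compares colors by exact RGBA channels and rotates 2D vectors by an angle in degrees using sine and cosine math expressions.
; It also finds the level's BP_UMGMapManager by searching all actors, printing a warning and returning none when it is missing, invalid or duplicated.
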(fn MarkerTagIsValid
  (params (In%20Tag :type String))
  (return (not (or (Utilities|Enum|Equal(Enum) In%20Tag "None") (Utilities|Enum|Equal(Enum) In%20Tag "")))))

(fn FindMapManager
  (Utilities|FlowControl|Sequence
    (:then_0
      (LocalVariables|SetOut%20Manager 0)
      (bind _outactors (Actor|GetAllActorsOfClass (LocalVariables|Get__WorldContext) "/Game/UMGMapCore/Blueprints/BP_UMGMapManager.BP_UMGMapManager_C"))
      (switch int (Utilities|Array|Length _outactors)
        (:Default
          (Development|PrintString 0 "Warning : Multiple Map Managers Found !" true true "(R=1.000000,G=0.461427,B=0.000000,A=1.000000)"))
        (:0
          (Development|PrintString 0 "Warning : Map Manager Not Found  !" true true "(R=1.000000,G=0.000000,B=0.000000,A=1.000000)"))
        (:1
          (Utilities|IsValid (Utilities|Array|Get(acopy) _outactors)
            (:Is%20Valid
              (LocalVariables|SetOut%20Manager (Utilities|Array|Get(acopy) _outactors)))
            (:Is%20Not%20Valid
              (Development|PrintString 0 "Warning : Map Manager Not Valid  !" true true "(R=1.000000,G=0.000000,B=0.000000,A=1.000000)"))))))
    (:then_1
      (return (LocalVariables|GetOut%20Manager)))))

(fn Equal
  (params (Color%20A :type Linear%20Color%20Structure) (Color%20B :type Linear%20Color%20Structure))
  (bind (_r _g _b _a) (Utilities|Struct|BreakLinearColor Color%20A))
  (bind (_r_2 _g_2 _b_2 _a_2) (Utilities|Struct|BreakLinearColor Color%20B))
  (return (Math|Boolean|ANDBoolean (== _r _r_2) (== _g _g_2) (== _b _b_2) (== _a _a_2))))

(fn NotEqual
  (params (Color%20A :type Linear%20Color%20Structure) (Color%20B :type Linear%20Color%20Structure))
  (bind _returnvalue (CallFunction|Equal Color%20A Color%20B (LocalVariables|Get__WorldContext)))
  (return (not _returnvalue)))

(fn RotateVector2D
  (params (In%20Vector%202D :type Vector%202D%20Structure) (Angle%20In%20Degrees :type Float%20%28single-precision%29))
  (bind _returnvalue (Math|Trig|DegreesToRadians Angle%20In%20Degrees))
  (bind (_x _y) (Math|Vector2D|BreakVector2D In%20Vector%202D))
  (return (Math|Vector2D|MakeVector2D (|((x*(cos(angle)))-(y*(sin(angle)))) _x _y _returnvalue) (|((x*(sin(angle)))+(y*(cos(angle)))) _x _y _returnvalue))))