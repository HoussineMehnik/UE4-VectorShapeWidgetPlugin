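; Marker component that puts its owning actor on the map by registering with the map manager.
; It registers after a zero-length delay on BeginPlay and unregisters on owner destruction or DestroyComponentSafe.
; Marker interface events and getters expose status, tag, icon appearance and out-of-range hiding, clamping opacity, scale and rotation offset.
; World position is owner location plus an offset, and rotation can add a selected owner rotation axis.
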(event Custom|On%20Onwer%20Actor%20Destroyed
  (params (DestroyedActor :type Actor%20Object%20Reference))
  ;[1 0 0.9675] Initialization
  (bind _map_manager_reference (Variables|Default|GetMap%20Manager%20Reference)
    (:then
      (Default|UnregisterMarkerObject _map_manager_reference self))
    (:else)))

(event Custom|Init
  ;[1 0 0.9675] Initialization
  (Utilities|FlowControl|Sequence
    (:then_0
      (bind _return_value (CallFunction|FindMapManager))
      (bind _output_get (Variables|Default|SetMap%20Manager%20Reference _return_value))
      (Utilities|IsValid _output_get
        (:Is%20Valid
          (Default|RegisterMarkerObject _output_get self))))
    (:then_1
      (Game|AssignOnDestroyed (Components|GetOwner) (delegate Custom|On%20Onwer%20Actor%20Destroyed)))))

(event Custom|Destroy%20Component%20Safe
  ;[1 0 0] Safe Destroy Event
  (bind _map_manager_reference (Variables|Default|GetMap%20Manager%20Reference)
    (:then
      (Default|UnregisterMarkerObject _map_manager_reference self))
    (:else
      _))
  (Components|DestroyComponent))

(event EventBeginPlay
  ;[1 0.06233 0] Begin Play
  (Utilities|FlowControl|Delay 0.0)
  (CallFunction|Init))

(event EventUpdateMarkerStatus
  (params (New%20Status :type Enum_MarkerStatus%20Enum :default "NewEnumerator0"))
  ;[0 0.2854 1] Marker Object Interface Events
  (Variables|Default|SetStatus New%20Status))

(event EventSetMarkerIconObject
  (params (New%20Icon%20Object :type Object%20Object%20Reference))
  ;[0 0.2854 1] Marker Object Interface Events
  (Variables|Default|SetIcon%20Object New%20Icon%20Object))

(event EventSetMarkerColor
  (params (New%20Color :type Linear%20Color%20Structure))
  ;[0 0.2854 1] Marker Object Interface Events
  (Variables|Default|SetIcon%20Color New%20Color))

(event EventSetMarkerOpacity
  (params (New%20Opacity :type Float%20%28single-precision%29))
  ;[0 0.2854 1] Marker Object Interface Events
  (Variables|Default|SetIcon%20Opacity (Math|Float|Clamp(Float) New%20Opacity)))

(event EventSetMarkerRotationAngle
  (params (New%20Rotation%20Angle :type Float%20%28single-precision%29))
  ;[0 0.2854 1] Marker Object Interface Events
  (Variables|Default|SetRotation%20Offset (Math|Float|ClampAngle New%20Rotation%20Angle -1.8e+02 1.8e+02)))

(event EventSetMarkerScale
  (params (New%20Scale :type Float%20%28single-precision%29))
  ;[0 0.2854 1] Marker Object Interface Events
  (Variables|Default|SetScale (Math|Float|Clamp(Float) New%20Scale 0.0 1e+01)))

(event EventSetMarkerHiddenwhenGettingOutOfRange
  (params (Value :type Boolean))
  ;[0 0.2854 1] Marker Object Interface Events
  (Variables|Default|SetHide%20When%20Getting%20Out%20Of%20Range Value))

(fn GetMarkerIconColor
  (return (Variables|Default|GetIcon%20Color)))

(fn GetMarkerIconObject
  (return (Variables|Default|GetIcon%20Object)))

(fn GetMarkerIconOpacity
  (return (Variables|Default|GetIcon%20Opacity)))

(fn GetMarkerRotationAngle
  (bind _returnvalue (Components|GetOwner))
  (bind _rotation_offset (Variables|Default|GetRotation%20Offset))
  (bind _returnvalue_2 (Transformation|GetActorRotation _returnvalue))
  (bind (_roll _pitch _yaw) (Math|Rotator|BreakRotator _returnvalue_2))
  (return (select (Variables|Default|GetUse%20Owner%20Rotation) (+ _rotation_offset (Utilities|Select :Index (Variables|Default|GetRotation%20Axis) :NewEnumerator0 _roll :NewEnumerator1 _pitch :NewEnumerator2 _yaw)) _rotation_offset)))

(fn GetMarkerScale
  (return (Variables|Default|GetScale)))

(fn GetMarkerStatus
  (return (Variables|Default|GetStatus)))

(fn GetMarkerTag
  (return (Variables|Default|GetUnique%20Tag)))

(fn GetMarkerWorldPosition
  (return (+ (Transformation|GetActorLocation (Components|GetOwner)) (Variables|Default|GetLocation%20Offset))))

(fn IsMarkerHidenwhenGettingOutOfRange
  (return (Variables|Default|GetHide%20When%20Getting%20Out%20Of%20Range)))